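; GA_FireBall is a gameplay ability that fires a projectile after a timed cast.
; On activation it sets the cast time, then casting callbacks drive the spellcast montage, jumping to its cast-end section on success.
; A one-shot gameplay event wait then times the release, spawning the projectile slightly above the avatar's location along its forward vector and ending the ability.
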(event `self.K2_ActivateAbility`
  (set `self.CastTime` 10.0))

(event `self.K2_OnEndAbility`
  (params (bWasCancelled :type Boolean)))

(event `self.OnCastingStarted`
  (`AbilityTask_PlayMontageAndWait.CreatePlayMontageAndWaitProxy` "None" "/Game/Characters/Animations/Casting/Retargeted_Spellcast_Montage.Retargeted_Spellcast_Montage"))

(event `self.OnCastingSucceded`
  (bind _returnvalue (`self.GetAvatarActorFromActorInfo`))
  (`AbilityTask_PlayMontageAndWait.CreatePlayMontageAndWaitProxy` "None" "/Game/Characters/Animations/Casting/Retargeted_Spellcast_Montage.Retargeted_Spellcast_Montage" 1.0 "CastTimeEnd" false
    (:`then`
      (`AbilityTask_WaitGameplayEvent.WaitGameplayEvent` (struct :`TagName` "GameplayCue.Event.AbilityTwo") null true
        (:`EventReceived`
          (`self.SpawnProjectile` (+ (`Actor.K2_GetActorLocation` _returnvalue) (0.0 0.0 40.0)) (`Actor.GetActorForwardVector` _returnvalue))
          (`self.K2_EndAbility`))))))