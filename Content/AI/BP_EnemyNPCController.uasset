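; AI controller for an enemy NPC that runs BT_Enemy on possess and feeds it sight perception.
; A sighted actor becomes TargetActor and the focus, sets HasLineOfSight and cancels the pending timer.
; Losing sight starts a LineOfSightTime timer that clears the target but not the focus.
; The timer writes false to a misspelled "HasLineeOfSight" key, so HasLineOfSight itself is never reset here.
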(event `self.AIPerception.OnTargetPerceptionUpdated`
  (params (Actor :type "Actor Object Reference") (Stimulus :type "AIStimulus Structure"))
  (bind _returnvalue (`AIPerceptionSystem.GetSenseClassForStimulus` Stimulus))
  (if (== _returnvalue "/Script/AIModule.AISense_Sight")
    (if (`.bSuccessfullySensed` (break `AIStimulus` Stimulus))
      (`BlackboardComponent.SetValueAsObject` (`self.Blackboard`) "TargetActor" Actor)
      (`BlackboardComponent.SetValueAsBool` (`self.Blackboard`) "HasLineOfSight" true)
      (`self.K2_SetFocus` Actor)
      (`KismetSystemLibrary.K2_ClearAndInvalidateTimerHandle` (`self.WatchTimer`))
      (else
        (bind _returnvalue_2 (`KismetSystemLibrary.K2_SetTimerDelegate` (delegate `ClearLineOfSight`) (`self.LineOfSightTime`) false true))
        (set `self.WatchTimer` _returnvalue_2)))))

(event `ClearLineOfSight`
  (`BlackboardComponent.SetValueAsObject` (`self.Blackboard`) "TargetActor" null)
  (`BlackboardComponent.SetValueAsBool` (`self.Blackboard`) "HasLineeOfSight" false))

(event `self.ReceivePossess`
  (params (PossessedPawn :type "Pawn Object Reference"))
  (`self.RunBehaviorTree` "/Game/AI/BehiavourTrees/BT_Enemy.BT_Enemy"))

(fn `UserConstructionScript`
  (`parent.UserConstructionScript`))