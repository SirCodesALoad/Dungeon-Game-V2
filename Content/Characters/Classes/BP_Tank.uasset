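; Tank player class that sets up its shield recharge ability, local UI and action bar on BeginPlay.
; It grants and activates GA_TankRechargeShieldHealth, then creates shield and HUD widgets for the locally controlled player.
; Releasing right mouse cancels ability input, stops the block montage and reactivates shield recharge a tick later.
; A trigger sphere shows hovering health bars, always marked hostile, for other DungeonCrawler characters in range and hides them on exit.
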(event `self.ReceiveBeginPlay`
  (bind _returnvalue (`AbilitySystemBlueprintLibrary.GetAbilitySystemComponent` null))
  (`parent.ReceiveBeginPlay`)
  (`|ExecutionSequence`
    (:`then_0`
      (`KismetSystemLibrary.DelayUntilNextTick`)
      (`AbilitySystemComponent.K2_GiveAbility` _returnvalue "/Game/Gameplay/Abilities/GA_TankRechargeShieldHealth.GA_TankRechargeShieldHealth_C" 0 -1)
      (`AbilitySystemComponent.TryActivateAbilityByClass` _returnvalue "/Game/Gameplay/Abilities/GA_TankRechargeShieldHealth.GA_TankRechargeShieldHealth_C" true)
      (if (`self.IsLocallyControlled`)
        (bind _returnvalue_2 (`|CreateWidget` "/Game/UI/WB_UIShieldHealth.WB_UIShieldHealth_C"))
        (bind _output_get (set `self.ShieldHealth Widget` _returnvalue_2))
        (`UserWidget.AddToViewport` _output_get 0)
        (`/Game/UI/WB_UIShieldHealth.UpdateOwningCharacter` _returnvalue_2 self)))
    (:`then_1`
      (if (`self.IsLocallyControlled`)
        (bind _returnvalue_3 (`|CreateWidget` "/Game/UI/WB_UIPlayerHUD.WB_UIPlayerHUD_C"))
        (bind _output_get_2 (set `self.Player HUD` _returnvalue_3))
        (`UserWidget.AddToViewport` _output_get_2 0)))
    (:`then_2`
      (`KismetSystemLibrary.DelayUntilNextTick`)
      (`|ExecutionSequence`
        (:`then_0`
          (message `/Game/UI/BPI_ActionBar.Update Action Bar Ability` (`self.GetController`) 0 (`|GetArrayItem` (`self.AbilityIcons`))))
        (:`then_1`
          (message `/Game/UI/BPI_ActionBar.Update Action Bar Ability` (`self.GetController`) 1 (`|GetArrayItem` (`self.AbilityIcons`) 1)))))))

(event `Key|RightMouseButton`
  (params (Key :type "Key Structure"))
  (bind _returnvalue (`AbilitySystemBlueprintLibrary.GetAbilitySystemComponent` null))
  (:`Released`
    (`AbilitySystemComponent.InputCancel` _returnvalue)
    (`self.StopAnimMontage` "/Game/Characters/Animations/SwordAndShieldReTarget/Tank_Block.Tank_Block")
    (`KismetSystemLibrary.DelayUntilNextTick`)
    (`AbilitySystemComponent.TryActivateAbilityByClass` _returnvalue "/Game/Gameplay/Abilities/GA_TankRechargeShieldHealth.GA_TankRechargeShieldHealth_C" true)))

(event `self.AddToHudSphereTrigger.OnComponentBeginOverlap`
  (params (OverlappedComponent :type "PrimitiveComponent Object Reference") (OtherActor :type "Actor Object Reference") (OtherComp :type "PrimitiveComponent Object Reference") (OtherBodyIndex :type Integer) (bFromSweep :type Boolean) (SweepResult :type "HitResult Structure (by ref)"))
  (if (`self.IsLocallyControlled`)
    (bind _asdungeon_crawler_character (cast `DungeonCrawlerCharacter` OtherActor))
    (if (!= _asdungeon_crawler_character self)
      (`/Game/UI/WB_UIPlayerHUD.Add Hovering HealthBar` (`self.Player HUD`) _asdungeon_crawler_character "Hostile"))))

(event `self.AddToHudSphereTrigger.OnComponentEndOverlap`
  (params (OverlappedComponent :type "PrimitiveComponent Object Reference") (OtherActor :type "Actor Object Reference") (OtherComp :type "PrimitiveComponent Object Reference") (OtherBodyIndex :type Integer))
  (if (`self.IsLocallyControlled`)
    (bind _asdungeon_crawler_character (cast `DungeonCrawlerCharacter` OtherActor))
    (if (!= _asdungeon_crawler_character self)
      (`/Game/UI/WB_UIPlayerHUD.HideHealthBar` (`self.Player HUD`) _asdungeon_crawler_character))))

(fn `UserConstructionScript`)