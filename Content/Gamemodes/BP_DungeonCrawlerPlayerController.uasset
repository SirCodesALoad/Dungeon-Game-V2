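; BP_DungeonCrawlerPlayerController is the dungeon crawler's player controller, managing the player's HUD widgets.
; On BeginPlay, only for the local controller, it creates the WB_UIActionBar widget, stores it and adds it to the viewport.
; Its update events forward ability icons to action bar slots and send health as a percentage and formatted text to a stats widget reference, which this graph never assigns.
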(event `self.ReceiveBeginPlay`
  (if (`self.IsLocalPlayerController`)
    (`|ExecutionSequence`
      (:`then_1`
        (bind _returnvalue (`|CreateWidget` "/Game/UI/WB_UIActionBar.WB_UIActionBar_C"))
        (bind _output_get (set `self.ActionBarRef` _returnvalue))
        (`UserWidget.AddToViewport` _output_get 0)))))

(event `/Game/UI/BPI_Stats.Update Health Display`
  (params (CurrentHealth :type "Float (double-precision)") (MaxHealth :type "Float (double-precision)"))
  (`/Game/UI/WB_UIHealthBar.UpdateHealth` (`self.Stats Ref`) (/ CurrentHealth MaxHealth) (`|FormatText` "{0} : {1}" CurrentHealth MaxHealth)))

(event `/Game/UI/BPI_ActionBar.Update Action Bar Ability`
  (params (AbilityIndex :type Integer) (AbilityIcon :type "Texture Object Reference"))
  (`/Game/UI/WB_UIActionBar.AssignAbility` (`self.ActionBarRef`) AbilityIndex AbilityIcon))

(fn `UserConstructionScript`)